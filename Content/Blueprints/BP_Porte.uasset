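; BP_Porte is an interactive door that shows a widget while something overlaps its Box component.
; Overlap begin and end toggle the widget's visibility.
; Interact hides the widget and plays a timeline that raises the Box along world Z.
; Each update adds a lerped 0–10 offset to the current location, so movement accumulates and total travel depends on update count.
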(event `self.Box.OnComponentBeginOverlap`
  (params (OverlappedComponent :type "PrimitiveComponent Object Reference") (OtherActor :type "Actor Object Reference") (OtherComp :type "PrimitiveComponent Object Reference") (OtherBodyIndex :type Integer) (bFromSweep :type Boolean) (SweepResult :type "HitResult Structure (by ref)"))
  (`SceneComponent.SetVisibility` (`self.Widget`) true false))

(event `self.Box.OnComponentEndOverlap`
  (params (OverlappedComponent :type "PrimitiveComponent Object Reference") (OtherActor :type "Actor Object Reference") (OtherComp :type "PrimitiveComponent Object Reference") (OtherBodyIndex :type Integer))
  (`SceneComponent.SetVisibility` (`self.Widget`) false false))

(event `/Game/Blueprints/BPI_Interact.Interact`
  (bind _box (`self.Box`))
  (bind (_returnvalue_x _returnvalue_y _returnvalue_z) (`KismetMathLibrary.BreakVector` (`SceneComponent.K2_GetComponentLocation` _box)))
  (`SceneComponent.SetVisibility` (`self.Widget`) false false)
  (bind (_direction _open) (`Timeline|Timeline`)
    (:`Update`
      (`SceneComponent.K2_SetWorldLocation` _box (`KismetMathLibrary.MakeVector` _returnvalue_x _returnvalue_y (+ (`KismetMathLibrary.Lerp` 0.0 10.0 _open) _returnvalue_z)) false false))))

(fn `UserConstructionScript`)