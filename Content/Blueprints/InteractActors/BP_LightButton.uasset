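; BP_LightButton is an interactable button for a light puzzle that toggles a linked set of lights.
; A box overlap shows and hides its widget, and Interact hides the widget before toggling each entry in LightArray.
; LightChecker then sets AllLightOn by scanning the array until it finds an unlit light.
; When all are lit, it calls LightEnigmaWin on the BP_GameInstance cached at BeginPlay.
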(event `self.ReceiveBeginPlay`
  (bind _asbp_game_instance (cast `/Game/Blueprints/BP_GameInstance` (`GameplayStatics.GetGameInstance`)))
  (set `self.As BP Game Instance` _asbp_game_instance))

(event `self.Box.OnComponentBeginOverlap`
  (params (OverlappedComponent :type "PrimitiveComponent Object Reference") (OtherActor :type "Actor Object Reference") (OtherComp :type "PrimitiveComponent Object Reference") (OtherBodyIndex :type Integer) (bFromSweep :type Boolean) (SweepResult :type "HitResult Structure (by ref)"))
  (`SceneComponent.SetVisibility` (`self.Widget`) true false))

(event `self.Box.OnComponentEndOverlap`
  (params (OverlappedComponent :type "PrimitiveComponent Object Reference") (OtherActor :type "Actor Object Reference") (OtherComp :type "PrimitiveComponent Object Reference") (OtherBodyIndex :type Integer))
  (`SceneComponent.SetVisibility` (`self.Widget`) false false))

(event `/Game/Blueprints/BPI/BPI_Interact.Interact`
  (`SceneComponent.SetVisibility` (`self.Widget`) false false)
  (`|ExecutionSequence`
    (:`then_0`
      (for _array_element (`self.LightArray`)
        (`/Game/Blueprints/InteractActors/BP_Light.toggle` _array_element)
        (`self.LightChecker`)))
    (:`then_1`
      (`self.LightChecker`)
      (if (`self.AllLightOn`)
        (`/Game/Blueprints/BP_GameInstance.LightEnigmaWin` (`self.As BP Game Instance`))))))

(fn `LightChecker`
  (for _array_element (`self.LightArray`)
    (if (`/Game/Blueprints/InteractActors/BP_Light.isOn?` _array_element)
      (set `self.AllLightOn` true)
      (else
        (set `self.AllLightOn` false)
        (break)))))

(fn `UserConstructionScript`)