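; BP_Player is the player Blueprint that picks up coins and collectibles, interacts with nearby objects and is destroyed by any damage.
; On overlap it passes coin and collectible components to its collect-coin and collect components.
; The Interact input messages the first overlapping actor that implements BPI_Interact.
; BeginPlay creates the main HUD widget and adds it to the viewport.
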(event `self.ReceiveActorBeginOverlap`
  (params (OtherActor :type "Actor Object Reference"))
  (bind _returnvalue (`self.GetComponentByClass` OtherActor "/Game/Blueprints/BPC_CollecibleComponent.BPC_CollecibleComponent_C"))
  (bind _returnvalue_2 (`self.GetComponentByClass` OtherActor "/Game/Blueprints/BPC_CoinComponent.BPC_CoinComponent_C"))
  (`|ExecutionSequence`
    (:`then_0`
      (`/Engine/EditorBlueprintResources/StandardMacros.IsValid` _returnvalue_2
        (:`Is Valid`
          (`/Game/Blueprints/BPC_CollectCoinComponent.Collect Coin` (`self.BPC_CollectCoinComponent`) _returnvalue_2))))
    (:`then_1`
      (`/Engine/EditorBlueprintResources/StandardMacros.IsValid` _returnvalue
        (:`Is Valid`
          (`/Game/Blueprints/BPC_CollectComponent.Collect` (`self.BPC_CollectComponent`) _returnvalue))))))

(event `self.ReceiveBeginPlay`
  (`parent.ReceiveBeginPlay`)
  (bind _returnvalue (`|CreateWidget` "/Game/Blueprints/BPW_MainHUD.BPW_MainHUD_C"))
  (`UserWidget.AddToViewport` _returnvalue 0))

(event `InputAction|Interact`
  (params (Key :type "Key Structure"))
  (:`Pressed`
    (for _array_element (`self.GetOverlappingActors` "/Script/Engine.Actor")
      (if (`KismetSystemLibrary.DoesImplementInterface` _array_element "/Game/Blueprints/BPI_Interact.BPI_Interact_C")
        (message `/Game/Blueprints/BPI_Interact.Interact` _array_element)
        (break)))))

(event `self.ReceiveAnyDamage`
  (params (Damage :type "Float (single-precision)") (DamageType :type "DamageType Object Reference") (InstigatedBy :type "Controller Object Reference") (DamageCauser :type "Actor Object Reference"))
  (`self.K2_DestroyActor`))

(fn `UserConstructionScript`
  (`parent.UserConstructionScript`))