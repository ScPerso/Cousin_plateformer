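; BP_Button is an interactable button that sets a global on flag when pressed.
; A box trigger shows and hides a widget as actors enter and leave.
; Interact hides the widget and plays a Timeline that sinks the Cube by adding a lerped offset to its current Z each update, so movement accumulates.
; Each update also sets IsbuttonOn on the BP_GameInstance cached at BeginPlay.
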(event `self.ReceiveBeginPlay`
  (bind _asbp_game_instance (cast `/Game/Blueprints/BP_GameInstance` (`GameplayStatics.GetGameInstance`)))
  (set `self.As BP Game Instance` _asbp_game_instance))

(event `self.Box.OnComponentBeginOverlap`
  (params (OverlappedComponent :type "PrimitiveComponent Object Reference") (OtherActor :type "Actor Object Reference") (OtherComp :type "PrimitiveComponent Object Reference") (OtherBodyIndex :type Integer) (bFromSweep :type Boolean) (SweepResult :type "HitResult Structure (by ref)"))
  (`SceneComponent.SetVisibility` (`self.Widget`) true false))

(event `self.Box.OnComponentEndOverlap`
  (params (OverlappedComponent :type "PrimitiveComponent Object Reference") (OtherActor :type "Actor Object Reference") (OtherComp :type "PrimitiveComponent Object Reference") (OtherBodyIndex :type Integer))
  (`SceneComponent.SetVisibility` (`self.Widget`) false false))

(event `/Game/Blueprints/BPI_Interact.Interact`
  (bind _cube (`self.Cube`))
  (bind (_returnvalue_x _returnvalue_y _returnvalue_z) (`KismetMathLibrary.BreakVector` (`SceneComponent.K2_GetComponentLocation` _cube)))
  (`SceneComponent.SetVisibility` (`self.Widget`) false false)
  (bind (_direction _open) (`Timeline|Timeline`)
    (:`Update`
      (`SceneComponent.K2_SetWorldLocation` _cube (`KismetMathLibrary.MakeVector` _returnvalue_x _returnvalue_y (+ (`KismetMathLibrary.Lerp` 0.0 -1.0 _open) _returnvalue_z)) false false)
      (set `/Game/Blueprints/BP_GameInstance.IsbuttonOn` true (`self.As BP Game Instance`)))))

(fn `UserConstructionScript`)